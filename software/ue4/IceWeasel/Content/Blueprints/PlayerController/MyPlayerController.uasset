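; Player controller for a team deathmatch game, handling team spawning, chat and the pause, team selection and scoreboard widgets.
; BeginPlay sorts PlayerStarts by team tag and creates the local chat window.
; SpawnPlayer replaces the pawn with a team character at a random team start, using server events for clients.
; Chat messages route through the server, but the team-colored broadcast loop is disconnected, so ReplicateChatMessage never delivers them.
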(event `self.ReceiveBeginPlay`
  (`|ExecutionSequence`
    (:`then_0`
      ;[1 1 1] Get Spawn Points
      (bind _outactors (`GameplayStatics.GetAllActorsOfClass` "/Script/Engine.PlayerStart"))
      (for _array_element _outactors
        (`|ExecutionSequence`
          (:`then_0`
            (if (== (`PlayerStart.PlayerStartTag` _array_element) "TeamB")
              (`KismetArrayLibrary.Array_Add` (`self.Team B Spawns`) _array_element)))
          (:`then_1`
            (if (== (`PlayerStart.PlayerStartTag` _array_element) "TeamA")
              (`KismetArrayLibrary.Array_Add` (`self.Team A Spawns`) _array_element))))))
    (:`then_1`
      (`KismetSystemLibrary.Delay` 0.2)
      (if (`self.IsLocalPlayerController`)
        (bind _returnvalue (`|CreateWidget` "/Game/Widgets/HUD/ChatWindow.ChatWindow_C" self))
        (bind _output_get (set `self.ChatWindowRef` _returnvalue))
        (`UserWidget.AddToViewport` _output_get 0)
        (`Border.SetBrushColor` :`self` (`/Game/Widgets/HUD/ChatWindow.MessageListBorder` _output_get)) ; Opacity = 0 (Invisible)
        (`Widget.SetVisibility` (`/Game/Widgets/HUD/ChatWindow.ChatInputTextBox` _output_get) "Hidden")))))

(event `Show Pause Menu`
  ;[1 1 1] Show / Hide Pause Menu
  (`UserWidget.AddToViewport` (`self.PauseMenuRef`) 0)
  (`self.DisableInput` (`GameplayStatics.GetPlayerPawn` 0) (`GameplayStatics.GetPlayerController` 0))
  (set `self.bShowMouseCursor` true)
  (`WidgetBlueprintLibrary.SetInputMode_GameAndUIEx` self)
  (set `self.PauseMenuActive` true))

(event `Hide Pause Menu`
  ;[1 1 1] Show / Hide Pause Menu
  (`Widget.RemoveFromParent` (`self.PauseMenuRef`))
  (`self.EnableInput` (`GameplayStatics.GetPlayerPawn` 0) (`GameplayStatics.GetPlayerController` 0))
  (set `self.bShowMouseCursor` false)
  (`WidgetBlueprintLibrary.SetInputMode_GameOnly` self)
  (set `self.PauseMenuActive` false))

(event `InputAction|Pause`
  (params (Key :type "Key Structure" :default "AnyKey"))
  ;[1 1 1] Show / Hide Pause Menu
  (:`Pressed`
    (`/Engine/EditorBlueprintResources/StandardMacros.IsValid` (`self.PauseMenuRef`)
      (:`Is Valid`
        _)
      (:`Is Not Valid`
        (bind _returnvalue (`|CreateWidget` "/Game/Widgets/PauseMenu/PauseMenu.PauseMenu_C" (`GameplayStatics.GetPlayerController` 0)))
        (set `self.PauseMenuRef` _returnvalue)))
    (if (`self.PauseMenuActive`)
      (`self.Hide Pause Menu`)
      (else
        (`self.Show Pause Menu`)))))

(event `Show Team Selection UI`
  ;[1 1 1] Team selection
  (`/Engine/EditorBlueprintResources/StandardMacros.IsValid` (`self.TeamSelectionRef`)
    (:`Is Valid`
      _)
    (:`Is Not Valid`
      (bind _returnvalue (`|CreateWidget` "/Game/Widgets/HUD/TeamSelection.TeamSelection_C" self))
      (set `self.TeamSelectionRef` _returnvalue)))
  (`UserWidget.AddToViewport` (`self.TeamSelectionRef`) 0)
  (`WidgetBlueprintLibrary.SetInputMode_UIOnlyEx` (`GameplayStatics.GetPlayerController` 0)))

(event `InputAction|Scoreboard`
  (params (Key :type "Key Structure" :default "AnyKey"))
  (bind _scoreboardref (`self.ScoreboardRef`))
  (bind _scoreboardref_2 (`self.ScoreboardRef`))
  ;[1 1 1] Show / Hide Scoreboard
  (:`Pressed`
    (`/Engine/EditorBlueprintResources/StandardMacros.FlipFlop`
      (:`A`
        (`/Engine/EditorBlueprintResources/StandardMacros.IsValid` _scoreboardref_2
          (:`Is Valid`
            _)
          (:`Is Not Valid`
            (bind _returnvalue (`|CreateWidget` "/Game/Widgets/HUD/Scoreboard.Scoreboard_C" self))
            (set `self.ScoreboardRef` _returnvalue)))
        (`/Game/Widgets/HUD/Scoreboard.ClearScoreboardEntries` (`self.ScoreboardRef`))
        (`/Game/Widgets/HUD/Scoreboard.Update Scoreboard` _scoreboardref)
        (`|ExecutionSequence`
          (:`then_0`
            (`/Game/Widgets/HUD/Scoreboard.SetTeamName` _scoreboardref 0 "Mannequin")
            (`/Game/Widgets/HUD/Scoreboard.SetTeamName` _scoreboardref 1 "Owen"))
          (:`then_1`
            (`UserWidget.AddToViewport` (`self.ScoreboardRef`) 0))))
      (:`B`
        (`/Engine/EditorBlueprintResources/StandardMacros.IsValid` _scoreboardref_2
          (:`Is Valid`
            (`Widget.RemoveFromParent` (`self.ScoreboardRef`))))))))

(event `InputAction|Chat`
  (params (Key :type "Key Structure" :default "AnyKey"))
  (bind _chatwindowref (`self.ChatWindowRef`))
  (bind _chatwindowref_2 (`self.ChatWindowRef`))
  (bind _chatinputtextbox (`/Game/Widgets/HUD/ChatWindow.ChatInputTextBox` _chatwindowref))
  (bind _messagelistborder (`/Game/Widgets/HUD/ChatWindow.MessageListBorder` _chatwindowref))
  (bind _messagelist (`/Game/Widgets/HUD/ChatWindow.MessageList` _chatwindowref))
  (bind _fadeout (`/Game/Widgets/HUD/ChatWindow.FadeOut` _chatwindowref_2))
  ;[1 1 1] Show / Hide Chat WIndow
  (:`Pressed`
    (`/Engine/EditorBlueprintResources/StandardMacros.FlipFlop`
      (:`A`
        (`Widget.SetVisibility` _chatinputtextbox "Visible") ; Show Input text box
        (`Border.SetBrushColor` _messagelistborder (`self.ChatBorderBrushColor`))
        (`Widget.SetVisibility` _messagelist "Visible") ; Show the message list
        (`UserWidget.StopAnimation` _chatwindowref_2 _fadeout) ; Stop the fadeout animation
        (`WidgetBlueprintLibrary.SetInputMode_GameAndUIEx` self (`/Game/Widgets/HUD/ChatWindow.ChatInputTextBox` (`self.ChatWindowRef`)))
        (set `self.ChatWindowActive` true))
      (:`B`
        (`Widget.SetVisibility` _chatinputtextbox "Hidden") ; Hide Input text box
        (`Border.SetBrushColor` :`self` _messagelistborder) ; Opacity = 0 (Invisible)
        (`Widget.SetVisibility` _messagelist "Hidden") ; Hide the message list
        (`UserWidget.StopAnimation` _chatwindowref_2 _fadeout) ; Stop the fadeout animation
        (`WidgetBlueprintLibrary.SetInputMode_GameOnly` self)
        (set `self.ChatWindowActive` false)))))

(event `Spawn Player`
  (params (Team :type Integer))
  (bind _returnvalue (`KismetSystemLibrary.IsServer`))
  (bind _returnvalue_2 (`self.K2_GetPawn`))
  ;[1 1 1] Team selection
  (switch `int` Team
    (:`0`
      (if _returnvalue
        (bind _spawnedcharacter (`self.SpawnTeamACharacter`))
        (`self.K2_DestroyActor` _returnvalue_2)
        (`self.Possess` _spawnedcharacter)
        (else
          (`self.Spawn Team A Character On Server` self))))
    (:`1`
      (if _returnvalue
        (bind _spawnedcharacter_2 (`self.SpawnTeamBCharacter`))
        (`self.K2_DestroyActor` _returnvalue_2)
        (`self.Possess` _spawnedcharacter_2)
        (else
          (`self.Spawn Team B Character On Server` self))))))

(event `Add Chat Message On Client`
  (params (Sender :type Text) (Message :type Text) (`Sender Text Color` :type "LinearColor Structure") (`Message Text Color` :type "LinearColor Structure"))
  ;[1 1 1] Chat system
  (`self.AddChatMessage` Sender Message `Sender Text Color` `Message Text Color`))

(event `Server Replicate Message`
  (params (Sender :type Text) (Message :type Text) (`Player Controller` :type "PlayerController Object Reference"))
  ;[1 1 1] Chat system
  (`self.ReplicateChatMessage` Sender Message `Player Controller`))

(event `Spawn Team A Character On Server`
  (params (`Player Controller` :type "PlayerController Object Reference"))
  ;[1 1 1] Team selection
  (bind _spawnedcharacter (`self.SpawnTeamACharacter`))
  (`self.K2_DestroyActor` (`self.K2_GetPawn` `Player Controller`))
  (`self.Possess` `Player Controller` _spawnedcharacter))

(event `Spawn Team B Character On Server`
  (params (`Player Controller` :type "PlayerController Object Reference"))
  ;[1 1 1] Team selection
  (bind _spawnedcharacter (`self.SpawnTeamBCharacter`))
  (`self.K2_DestroyActor` (`self.K2_GetPawn` `Player Controller`))
  (`self.Possess` `Player Controller` _spawnedcharacter))

(fn `AddChatMessage`
  (params (Sender :type Text) (Message :type Text) (`Sender Text Color` :type "LinearColor Structure") (`Message Text Color` :type "LinearColor Structure"))
  (bind _chatwindowref (`self.ChatWindowRef`))
  (bind _chatwindowref_2 (`self.ChatWindowRef`))
  (`/Engine/EditorBlueprintResources/StandardMacros.IsValid` _chatwindowref
    (:`Is Valid`
      (if (`self.ChatWindowActive`)
        (`Widget.SetVisibility` (`/Game/Widgets/HUD/ChatWindow.MessageList` _chatwindowref_2) "Visible") ; Don't play fadeout animation in case the chat window is already\nactive - just add the message to the window
        (else
          (`UserWidget.PlayAnimation` _chatwindowref_2 (`/Game/Widgets/HUD/ChatWindow.FadeOut` _chatwindowref) 0.0 1 "Forward" 1.0) ; When a message is received,\nshow the message and play the fadeout animation\n\n(The animation handles showing of the message aswell)
        ))
      (`/Game/Widgets/HUD/ChatWindow.AddChatMessage` (`self.ChatWindowRef`) Sender Message `Sender Text Color` `Message Text Color`))))

(fn `ReplicateChatMessage`
  (params (Sender :type Text) (Message :type Text) (`Player Controller` :type "PlayerController Object Reference"))
  (locals (SenderText :type Text) (MessageText :type Text))
  (`|ExecutionSequence`
    (:`then_0`
      (set `local.SenderText` Sender)
      (set `local.MessageText` Message))
    (:`then_1`
      (bind _asmy_team_death_match (cast `/Game/Blueprints/GameMode/MyTeamDeathMatch` (`GameplayStatics.GetGameMode`))))))

(fn `SpawnTeamACharacter`
  (returns (SpawnedCharacter :type "Character Object Reference"))
  (bind _team_a_spawns (`self.Team A Spawns`))
  (bind _returnvalue (`|SpawnActorFromClass` "/Game/Blueprints/Characters/MyBaseCharacter.MyBaseCharacter_C" (`self.GetTransform` (`KismetArrayLibrary.Array_Get` _team_a_spawns (`KismetMathLibrary.RandomInteger` (`KismetArrayLibrary.Array_Length` _team_a_spawns)))) "AdjustIfPossibleButAlwaysSpawn" "OverrideRootScale"))
  (return _returnvalue))

(fn `SpawnTeamBCharacter`
  (returns (SpawnedCharacter :type "Character Object Reference"))
  (bind _team_b_spawns (`self.Team B Spawns`))
  (bind _returnvalue (`|SpawnActorFromClass` "/Game/Blueprints/Characters/Owen.Owen_C" (`self.GetTransform` (`KismetArrayLibrary.Array_Get` _team_b_spawns (`KismetMathLibrary.RandomInteger` (`KismetArrayLibrary.Array_Length` _team_b_spawns)))) "AdjustIfPossibleButAlwaysSpawn" "OverrideRootScale"))
  (return _returnvalue))

(fn `UserConstructionScript`)