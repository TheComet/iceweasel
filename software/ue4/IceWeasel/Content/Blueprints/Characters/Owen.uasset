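; Owen is a character Blueprint, derived from a parent class, that sets up which body mesh holds its weapon.
; On BeginPlay it runs the parent logic, waits briefly, then checks whether the character is locally controlled.
; The weapon mesh snaps to the right-hand socket on the first-person view mesh for local control, or on the main mesh otherwise.
; The construction script only calls the parent, and Tick is disabled.
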(event `self.ReceiveBeginPlay`
  (`parent.ReceiveBeginPlay`)
  (`KismetSystemLibrary.Delay` 0.2)
  (if (`self.IsLocallyControlled`)
    (`SceneComponent.K2_AttachToComponent` (`self.WeaponMesh`) (`self.FirstPersonViewMesh`) "RightHandWeaponSocket" "SnapToTarget" "SnapToTarget" "SnapToTarget" true)
    (else
      (`SceneComponent.K2_AttachToComponent` (`self.WeaponMesh`) (`self.Mesh`) "RightHandWeaponSocket" "SnapToTarget" "SnapToTarget" "SnapToTarget" true))))

(fn `UserConstructionScript`
  (`parent.UserConstructionScript`))