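; GravityScaleZone is a trigger volume actor that changes a Character's gravity and air control while it is inside.
; On box begin overlap it sets the character's movement GravityScale to EnterGravityScale and grants partial air control.
; On end overlap it sets GravityScale to ExitGravityScale and zeroes air control, rather than restoring the character's previous values.
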(event `self.Box.OnComponentBeginOverlap`
  (params (OverlappedComponent :type "PrimitiveComponent Object Reference") (OtherActor :type "Actor Object Reference") (OtherComp :type "PrimitiveComponent Object Reference") (OtherBodyIndex :type Integer) (bFromSweep :type Boolean) (SweepResult :type "HitResult Structure (by ref)"))
  (bind _ascharacter (cast `Character` OtherActor))
  (`/Engine/EditorBlueprintResources/StandardMacros.IsValid` _ascharacter
    (:`Is Valid`
      (bind _charactermovement (`Character.CharacterMovement` _ascharacter))
      (set `CharacterMovementComponent.GravityScale` (`self.Enter Gravity Scale`) _charactermovement)
      (set `CharacterMovementComponent.AirControl` 0.4 _charactermovement))))

(event `self.Box.OnComponentEndOverlap`
  (params (OverlappedComponent :type "PrimitiveComponent Object Reference") (OtherActor :type "Actor Object Reference") (OtherComp :type "PrimitiveComponent Object Reference") (OtherBodyIndex :type Integer))
  (bind _ascharacter (cast `Character` OtherActor))
  (`/Engine/EditorBlueprintResources/StandardMacros.IsValid` _ascharacter
    (:`Is Valid`
      (bind _charactermovement (`Character.CharacterMovement` _ascharacter))
      (set `CharacterMovementComponent.GravityScale` (`self.Exit Gravity Scale`) _charactermovement)
      (set `CharacterMovementComponent.AirControl` 0.0 _charactermovement))))

(fn `UserConstructionScript`)