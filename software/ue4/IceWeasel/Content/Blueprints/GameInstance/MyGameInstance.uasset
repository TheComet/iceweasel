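; Game Instance that handles multiplayer session matchmaking: finding, joining, hosting and destroying sessions, plus printing network and travel errors.
; FindandJoinMatch resets state, searches sessions, joins the lowest-ping one that isn't full, and records the search outcome in FoundSessionType.
; Searching and hosting both fire DestroySessionCaller first, without waiting for its result.
; HostMatch only creates the session and opens no level; helper functions turn failure enums into printed messages.
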(event `self.HandleNetworkError`
  (params (FailureType :type "ENetworkFailure Enum" :default "NetDriverAlreadyExists") (bIsServer :type Boolean))
  ;[1 1 1] Handle net errors
  (`KismetSystemLibrary.PrintString` (`self.NetErrorToString` FailureType) true true (struct :`R` 1.0 :`B` 0.016751 :`A` 1.0) 5.0))

(event `self.HandleTravelError`
  (params (FailureType :type "ETravelFailure Enum" :default "NoLevel"))
  ;[1 1 1] Handle travel errors
  (`KismetSystemLibrary.PrintString` (`self.TravelErrorToString` FailureType) true true (struct :`R` 0.863157 :`G` 0.1025 :`A` 1.0) 5.0))

(event `ResetVariables`
  ;[1 1 1] Variables to reset before finding the match
  (set `self.FoundJoinableSession` false)
  (set `self.JoinableSessionIndex` 0)
  (set `self.PingMax` 999999)
  (set `self.FoundSessionType` "NewEnumerator4")
  (`self.Destroy Session Caller`))

(event `Find and Join Match`
  (bind _item (`KismetArrayLibrary.Array_Get` (`self.SessionsFound`) (`self.JoinableSessionIndex`)))
  ;[1 1 1] Find and Join a Match (if possible)
  (`self.ResetVariables`)
  (bind _results (`FindSessionsCallbackProxy.FindSessions` (`GameplayStatics.GetPlayerController` 0) (`self.MaxSessionResults`) (`self.UseLAN?`))
    (:`OnSuccess`
      (bind _output_get (set `self.SessionsFound` _results))
      (bind _returnvalue (`KismetArrayLibrary.Array_Length` _output_get))
      (`KismetSystemLibrary.PrintString` (`KismetTextLibrary.Conv_TextToString` (`|FormatText` "Found Sessions: {s}" _returnvalue)))
      (if (!= _returnvalue 0)
        (for (_array_element _array_index) (`self.SessionsFound`)
          (bind _returnvalue_2 (`FindSessionsCallbackProxy.GetPingInMs` _array_element))
          (if (<= _returnvalue_2 (`self.PingMax`))
            (bind _returnvalue_3 (`FindSessionsCallbackProxy.GetCurrentPlayers` _array_element))
            (bind _returnvalue_4 (`FindSessionsCallbackProxy.GetMaxPlayers` _array_element))
            (if (!= _returnvalue_3 _returnvalue_4)
              (set `self.PingMax` _returnvalue_2)
              (set `self.JoinableSessionIndex` _array_index)
              (set `self.FoundJoinableSession` true)))
          (`KismetSystemLibrary.PrintString` (`KismetStringLibrary.Concat_StrStr` "Found a session with ping: " (`KismetStringLibrary.Conv_IntToString` _returnvalue_2) " and Current / Max Players: " (`KismetStringLibrary.Conv_IntToString` _returnvalue_3) "/" (`KismetStringLibrary.Conv_IntToString` _returnvalue_4)) true true (struct :`G` 0.16113 :`B` 1.0 :`A` 1.0) 30.0))
        (if (`self.FoundJoinableSession`)
          (set `self.FoundSessionType` "NewEnumerator0")
          (`self.Join Match` _item)
          (set `self.Current Session` _item)
          (else
            (set `self.FoundSessionType` "NewEnumerator1")))
        (else
          (set `self.FoundSessionType` "NewEnumerator3"))))
    (:`OnFailure`
      (`KismetSystemLibrary.PrintString` "Find Session: FAILED")
      (set `self.FoundSessionType` "NewEnumerator2"))))

(event `Join Match`
  (params (Session :type "BlueprintSessionResult Structure"))
  ;[1 1 1] Join Match / Join Session
  (`JoinSessionCallbackProxy.JoinSession` (`GameplayStatics.GetPlayerController` 0) Session
    (:`OnSuccess`
      (`KismetSystemLibrary.PrintString` "Join Session: SUCCESS")
      (`WidgetBlueprintLibrary.SetInputMode_GameOnly` (`GameplayStatics.GetPlayerController` 0)))
    (:`OnFailure`
      (`KismetSystemLibrary.PrintString` "Join Session: FAILED"))))

(event `Host Match`
  ;[1 1 1] Host Match / Create Session
  (`self.Destroy Session Caller`)
  (`CreateSessionCallbackProxy.CreateSession` (`GameplayStatics.GetPlayerController` 0) (`self.MaxPlayers`) (`self.UseLAN?`)
    (:`OnSuccess`
      (`KismetSystemLibrary.PrintString` "Create Session: SUCCESS"))
    (:`OnFailure`
      (`KismetSystemLibrary.PrintString` "Create Session: FAILED"))))

(event `Destroy Session Caller`
  ;[1 1 1] Destroy Session - Should be called before finding/hosting match and when leaving a game/session
  (`DestroySessionCallbackProxy.DestroySession` (`GameplayStatics.GetPlayerController` 0)
    (:`OnSuccess`
      (`KismetSystemLibrary.PrintString` "Session Destroyed Successfully"))
    (:`OnFailure`
      (`KismetSystemLibrary.PrintString` "Failed to Destroy Session"))))

(fn `NetErrorToString`
  (params (Error :type "ENetworkFailure Enum"))
  (returns (OutString :type String))
  (locals (ErrorString :type String))
  (switch `ENetworkFailure` Error
    (:`NetDriverAlreadyExists`
      (set `local.ErrorString` "Error: lost connection to host." :!label _label))
    (:`NetDriverCreateFailure`
      (goto _label))
    (:`NetDriverListenFailure`
      (goto _label))
    (:`ConnectionLost`
      (goto _label))
    (:`ConnectionTimeout`
      (set `local.ErrorString` "Error: connection timed out."))
    (:`FailureReceived`
      (goto _label))
    (:`OutdatedClient`
      (goto _label))
    (:`OutdatedServer`
      (goto _label))
    (:`PendingConnectionFailure`
      (goto _label))
    (:`NetGuidMismatch`
      (goto _label))
    (:`NetChecksumMismatch`
      (goto _label)))
  (return (`local.ErrorString`)))

(fn `TravelErrorToString`
  (params (Error :type "ETravelFailure Enum"))
  (returns (OutString :type String))
  (return (`KismetStringLibrary.Concat_StrStr` "Error: failed to travel. " (`|GetEnumeratorNameAsString` Error))))